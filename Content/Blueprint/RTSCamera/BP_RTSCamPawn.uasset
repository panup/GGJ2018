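; RTS-style camera pawn with cursor-based tool use, in which tool 2 places gas actors in the world.
; Axis inputs move the pawn, the mouse wheel zooms the spring arm, and holding right mouse hides the cursor and opens gates for yaw and camera pitch.
; Number keys select four tools, but only tool 2 acts: while SetDestination opens a Tick gate, a Delay throttles BP_Gas spawning under the cursor until GasCountVariable runs out.
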(event EventBeginPlay
  (Variables|/Script/Engine.PlayerController|SetbShowMouseCursor (Game|GetPlayerController 0) true))

(event Collision|EventActorBeginOverlap
  (params (OtherActor :type Actor%20Object%20Reference)))

(event EventTick
  (params (DeltaSeconds :type Float%20%28single-precision%29))
  (bind _returnvalue (Game|GetPlayerController 0))
  (bind _gascountvariable (Variables|Default|GetGasCountVariable))
  (Utilities|FlowControl|Gate true
    (:Exit
      (if (Game|Player|IsInputKeyDown _returnvalue (stale Input|ActionEvents|InputActionSetDestination Key))
        (switch int (Variables|Default|GetSelectedTool)
          (:2
            (Utilities|FlowControl|Delay 0.2)
            (if (> _gascountvariable 0)
              (bind _result (Math|Integer|DecrementInt _gascountvariable)
                (:%20%20
                  (Development|PrintString (Utilities|String|Append "Gas Count: " (Utilities|String|ToString(Integer) _result)))
                  (CallFunction|SpawntoHitLocation (.HitResult (Game|Player|GetHitResultUnderCursorbyChannel _returnvalue "TraceTypeQuery1" true))))))))))))

(event Input|ActionEvents|InputActionSelectedTool
  (params (Key :type Key%20Structure))
  (:Pressed
    (switch int (Utilities|String|GetCharacterasNumber (Utilities|String|ToString(Text) (Class|KismetInputLibrary|KeyGetDisplayName Key)))
      (:49
        (Variables|Default|SetSelectedTool 1))
      (:50
        (Variables|Default|SetSelectedTool 2))
      (:51
        (Variables|Default|SetSelectedTool 3))
      (:52
        (Variables|Default|SetSelectedTool 4)))))

(event Input|ActionEvents|InputActionSetDestination
  (params (Key :type Key%20Structure))
  (bind _returnvalue (Game|GetPlayerController 0))
  (bind _gascountvariable (Variables|Default|GetGasCountVariable))
  (:Pressed
    (Utilities|FlowControl|Gate true) ; enters at Open
  )
  (:Released
    (Utilities|FlowControl|Gate true) ; enters at Close
  ))

(event Input|AxisEvents|InputAxisMoveForward
  (params (AxisValue :type Float%20%28single-precision%29))
  (Transformation|AddActorLocalOffset (Math|Vector|MakeVector (* AxisValue (Variables|Default|GetMoveSpeed)) 0.0 0.0) false false))

(event Input|AxisEvents|InputAxisMoveRight
  (params (AxisValue :type Float%20%28single-precision%29))
  (Transformation|AddActorLocalOffset (Math|Vector|MakeVector 0.0 (* AxisValue (Variables|Default|GetMoveSpeed)) 0.0) false false))

(event Input|MouseEvents|MouseX
  (params (AxisValue :type Float%20%28single-precision%29))
  (Utilities|FlowControl|Gate true
    (:Exit
      (Transformation|AddActorLocalRotation (Math|Rotator|MakeRotator 0.0 0.0 (* AxisValue (Variables|Default|GetRotateSpeed))) false false))))

(event Input|MouseEvents|MouseY
  (params (AxisValue :type Float%20%28single-precision%29))
  (Utilities|FlowControl|Gate true
    (:Exit
      (Transformation|AddLocalRotation (Variables|Default|GetCamera) (Math|Rotator|MakeRotator 0.0 (* AxisValue (Variables|Default|GetRotateSpeed)) 0.0) false false))))

(event Input|MouseEvents|MouseWheelDown
  (params (Key :type Key%20Structure))
  (bind _springarm (Variables|Default|GetSpringArm))
  (:Pressed
    (Variables|/Script/Engine.SpringArmComponent|SetTargetArmLength _springarm (+ (Variables|/Script/Engine.SpringArmComponent|GetTargetArmLength _springarm) 5e+01))))

(event Input|MouseEvents|MouseWheelUp
  (params (Key :type Key%20Structure))
  (bind _springarm (Variables|Default|GetSpringArm))
  (:Pressed
    (Variables|/Script/Engine.SpringArmComponent|SetTargetArmLength _springarm (- (Variables|/Script/Engine.SpringArmComponent|GetTargetArmLength _springarm) 5e+01))))

(event Input|MouseEvents|RightMouseButton
  (params (Key :type Key%20Structure))
  (bind _returnvalue (Game|GetPlayerController 0))
  (:Pressed
    (Variables|/Script/Engine.PlayerController|SetbShowMouseCursor _returnvalue false)
    (Utilities|FlowControl|Sequence
      (:then_0
        (Utilities|FlowControl|Gate true) ; enters at Open
      )
      (:then_1
        (Utilities|FlowControl|Gate true) ; enters at Open
      )))
  (:Released
    (Variables|/Script/Engine.PlayerController|SetbShowMouseCursor _returnvalue true)
    (Utilities|FlowControl|Sequence
      (:then_0
        (Utilities|FlowControl|Gate true) ; enters at Close
      )
      (:then_1
        (Utilities|FlowControl|Gate true) ; enters at Close
      ))))

(event Input|MouseEvents|LeftMouseButton
  (params (Key :type Key%20Structure))
  (:Pressed
    (switch int (Variables|Default|GetSelectedTool)
      (:2
        (if (<= (Variables|Default|GetGasCountVariable) 0)
          _)))))

(fn ConstructionScript)

(fn SpawntoHitLocation
  (params (HitResult :type Hit%20Result%20Structure))
  (Game|SpawnActorfromClass "/Game/Blueprint/Onion/BP_Gas.BP_Gas_C" (Math|Conversions|ToTransform(Vector) (.Location (Collision|BreakHitResult HitResult))) "Undefined" 0 0))