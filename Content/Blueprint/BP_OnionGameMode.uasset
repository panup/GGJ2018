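; BP_OnionGameMode is a game mode that provides a countdown and an infection measure for BP_Onion actors.
; The Countdown event plays a timeline from the start and prints its current value on each update.
; InfectedPercentage gathers every BP_Onion, counts those flagged as infected, and returns their share of the total as a fraction.
; BeginPlay and Tick are unused, and nothing in this Blueprint calls either the countdown or the percentage function.
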(event Custom|Countdown
  (bind _countdowner (Timeline|CountdownTimeline PlayFromStart)
    (:Update
      (Development|PrintString (Utilities|String|ToString(Float) _countdowner)))))

(event EventBeginPlay)

(event EventTick
  (params (DeltaSeconds :type Float%20%28single-precision%29)))

(fn ConstructionScript)

(fn InfectedPercentage
  (bind _outactors (Actor|GetAllActorsOfClass "/Game/Blueprint/Onion/BP_Onion.BP_Onion_C"))
  (for _array_element _outactors
    (if (Variables|/Game/Blueprint/Onion/BP_Onion.BP_Onion_C|GetIsInfected _array_element)
      (Math|Integer|IncrementInt (LocalVariables|GetInfectedCount))))
  (return (/ (Math|Conversions|ToFloat(Integer) (LocalVariables|GetInfectedCount)) (Math|Conversions|ToFloat(Integer) (Utilities|Array|Length _outactors)))))