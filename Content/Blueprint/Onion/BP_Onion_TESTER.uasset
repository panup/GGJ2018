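; BP_Onion_TESTER is a test onion actor for an infection mechanic, shown by swapping between normal and red onion materials.
; The construction script picks the mesh material from IsInfected.
; On overlap, an infected onion turns another tester onion red, then prints the infected percentage from BP_OnionGameMode.
; The overlap changes only the material, leaving the other onion's IsInfected flag untouched.
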(event EventBeginPlay
  (|CallParentFunction) ; This node is disabled and will not be called.\nDrag off pins to build functionality.
)

(event Collision|EventActorBeginOverlap
  (params (OtherActor :type Actor%20Object%20Reference))
  (|CallParentFunction OtherActor)
  (if (Variables|Default|GetIsInfected)
    (bind _asbp_onion_tester (Utilities|Casting|CastToBP_Onion_TESTER OtherActor))
    (Rendering|Material|SetMaterial (Variables|/Script/Engine.Character|GetMesh _asbp_onion_tester) 0 "/Game/Meshes/MAT_RedOnion.MAT_RedOnion")
    (bind _asbp_onion_game_mode (Utilities|Casting|CastToBP_OnionGameMode (Game|GetGameMode)))
    (bind _percentage (Default|InfectedPercentage _asbp_onion_game_mode))
    (Development|PrintString (Utilities|String|ToString(Float) _percentage))))

(event EventTick
  (params (DeltaSeconds :type Float%20%28single-precision%29))
  (|CallParentFunction DeltaSeconds) ; This node is disabled and will not be called.\nDrag off pins to build functionality.
)

(fn ConstructionScript
  (bind _mesh (Variables|Character|GetMesh))
  (|CallParentFunction)
  (if (Variables|Default|GetIsInfected)
    (Rendering|Material|SetMaterial _mesh 0 "/Game/Meshes/MAT_RedOnion.MAT_RedOnion")
    (else
      (Rendering|Material|SetMaterial _mesh 0 "/Game/Meshes/MAT_Onion.MAT_Onion"))))